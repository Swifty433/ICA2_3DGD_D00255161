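; Interactable phone actor that the player repairs with inventory items before it can be used.
; InteractwithObject steps through PhoneRepairStage, consuming a fuse and then a coin from the first-person character's inventory with voice and sound feedback, then opens the WBP_PhoneKeypad widget in UI-only input.
; Hover events toggle custom depth on the mesh for highlighting.
; A separate E-key FlipFlop plays or stops the phone audio, but the collision box's input toggling is disconnected.
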(event `self.CollisionBox.OnComponentBeginOverlap`
  (params (OverlappedComponent :type "PrimitiveComponent Object Reference") (OtherActor :type "Actor Object Reference") (OtherComp :type "PrimitiveComponent Object Reference") (OtherBodyIndex :type Integer) (bFromSweep :type Boolean) (SweepResult :type "HitResult Structure (by ref)"))
  ;[0.9323 0.08657 0.2343 0.5] Player Input on and off if in collison box
)

(event `self.CollisionBox.OnComponentEndOverlap`
  (params (OverlappedComponent :type "PrimitiveComponent Object Reference") (OtherActor :type "Actor Object Reference") (OtherComp :type "PrimitiveComponent Object Reference") (OtherBodyIndex :type Integer))
  ;[0.9323 0.08657 0.2343 0.5] Player Input on and off if in collison box
)

(event `Key|E`
  (params (Key :type "Key Structure"))
  ;[0 1 0.6698 0.5] On or off for the audio component
  (:`Pressed`
    (`/Engine/EditorBlueprintResources/StandardMacros.FlipFlop`
      (:`A`
        (`AudioComponent.Play` (`self.PhoneAudio`) 0.0)
        (`KismetSystemLibrary.PrintString` "Object Interacted" true true (struct :`G` 0.763156 :`B` 1.0 :`A` 1.0)))
      (:`B`
        (`AudioComponent.Stop` (`self.PhoneAudio`))
        (`KismetSystemLibrary.PrintString` "Object stopped" true true (struct :`G` 0.763156 :`B` 1.0 :`A` 1.0))))))

(event `/Game/3DGD/BluePrints/Interfaces/BPI_Interactable.InteractWithObject`
  (bind _returnvalue (`GameplayStatics.GetPlayerController` 0))
  ; Inventory logic for fixing the phone
  (bind _asbp_first_person_character (cast `/Game/FirstPerson/Blueprints/BP_FirstPersonCharacter` (`GameplayStatics.GetPlayerCharacter` 0)))
  (switch `int` (`self.PhoneRepairStage`)
    (:`0`
      (bind _playerinventory (`/Game/FirstPerson/Blueprints/BP_FirstPersonCharacter.PlayerInventory` _asbp_first_person_character))
      (if (`KismetArrayLibrary.Array_Contains` _playerinventory "NewEnumerator1")
        (`KismetArrayLibrary.Array_RemoveItem` _playerinventory "NewEnumerator1")
        (set `self.PhoneRepairStage` 1)
        (`GameplayStatics.PlaySound2D` "/Game/3DGD/AudioImplementation/SoundEffects/SelfMade/Dialogue/Player_Dialogue/NiceNowNeedCoin.NiceNowNeedCoin" 1.0 1.0 0.0 null null)
        (`KismetSystemLibrary.PrintString` "Nice i replaced the fuze but now i need a coin")
        (else
          (`GameplayStatics.PlaySound2D` "/Game/3DGD/AudioImplementation/SoundEffects/SelfMade/Dialogue/Player_Dialogue/PhoneBroken.PhoneBroken" 1.0 1.0 0.0 null null)
          (`KismetSystemLibrary.PrintString` "Looks like the fuze is blown")))
      (`GameplayStatics.PlaySound2D` "/Game/3DGD/AudioImplementation/SoundEffects/SelfMade/Other/zap.zap" 1.0 1.0 0.0 null null))
    (:`1`
      (if (`KismetArrayLibrary.Array_Contains` _playerinventory "NewEnumerator0")
        (`KismetArrayLibrary.Array_RemoveItem` _playerinventory "NewEnumerator0")
        (set `self.PhoneRepairStage` 2)
        (`GameplayStatics.PlaySound2D` "/Game/3DGD/AudioImplementation/SoundEffects/SelfMade/Dialogue/Player_Dialogue/Works_Now.Works_Now" 1.0 1.0 0.0 null null)
        (`KismetSystemLibrary.PrintString` "Nice the phone is fixed")
        (`GameplayStatics.PlaySound2D` "/Game/3DGD/AudioImplementation/SoundEffects/Sourced/Coin/CoinInsert.CoinInsert" 1.0 1.0 0.0 null null)
        (else
          (`GameplayStatics.PlaySound2D` "/Game/3DGD/AudioImplementation/SoundEffects/SelfMade/Dialogue/Player_Dialogue/NeedCoin.NeedCoin" 1.0 1.0 0.0 null null)
          (`KismetSystemLibrary.PrintString` "i need a coin to operate the phone"))))
    (:`2`
      ; Opening up the UI if items are held
      (set `PlayerController.bShowMouseCursor` true _returnvalue)
      (`WidgetBlueprintLibrary.SetInputMode_UIOnlyEx` _returnvalue null)
      (bind _returnvalue_2 (`|CreateWidget` "/Game/3DGD/UI/WBP/WBP_PhoneKeypad.WBP_PhoneKeypad_C"))
      (`UserWidget.AddToViewport` _returnvalue_2 0)
      (`GameplayStatics.GetAllActorsOfClass` "/Game/3DGD/AudioImplementation/Blueprints/BP_LightFlicker.BP_LightFlicker_C"))))

(event `/Game/3DGD/BluePrints/Interfaces/BPI_Interactable.UnHover`
  ; Hover event
  (`PrimitiveComponent.SetRenderCustomDepth` (`self.PhoneMesh`) false))

(event `/Game/3DGD/BluePrints/Interfaces/BPI_Interactable.OnHover`
  ; Hover event
  (`PrimitiveComponent.SetRenderCustomDepth` (`self.PhoneMesh`) true))

(fn `UserConstructionScript`)