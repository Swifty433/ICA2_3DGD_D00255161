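; Interactable cassette player actor that plays an audio clue when the player interacts with it while holding the required inventory item.
; Interaction checks the first-person character's inventory, then either restarts the clue sound via a stored audio component or plays a "need cassette" sound.
; Hover events toggle custom depth on the cube mesh for highlighting.
; Debug strings print on each interaction.
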(event `/Game/3DGD/BluePrints/Interfaces/BPI_Interactable.InteractWithObject`
  (bind _activetapeaudio (`self.ActiveTapeAudio`))
  ; Logic for cassette player
  (`GameplayStatics.PlaySound2D` null 1.0 1.0 0.0 null null)
  (`KismetSystemLibrary.PrintString` "Object Interacted" true true (struct :`G` 0.763156 :`B` 1.0 :`A` 1.0))
  (bind _asbp_first_person_character (cast `/Game/FirstPerson/Blueprints/BP_FirstPersonCharacter` (`GameplayStatics.GetPlayerCharacter` 0)))
  (if (`KismetArrayLibrary.Array_Contains` (`/Game/FirstPerson/Blueprints/BP_FirstPersonCharacter.PlayerInventory` _asbp_first_person_character) "NewEnumerator3")
    (`/Engine/EditorBlueprintResources/StandardMacros.IsValid` _activetapeaudio
      (:`Is Valid`
        (`AudioComponent.Stop` _activetapeaudio))
      (:`Is Not Valid`
        _))
    (bind _returnvalue (`GameplayStatics.SpawnSound2D` "/Game/3DGD/AudioImplementation/SoundEffects/SelfMade/Dialogue/Recorded_lines/CassetteAudioClue.CassetteAudioClue" 1.0 1.0 0.0 null))
    (set `self.ActiveTapeAudio` _returnvalue)
    (`KismetSystemLibrary.PrintString` "hehehehehe")
    (else
      (`GameplayStatics.PlaySound2D` "/Game/3DGD/AudioImplementation/SoundEffects/SelfMade/Dialogue/Player_Dialogue/NeedCassette.NeedCassette" 1.0 1.0 0.0 null null)
      (`KismetSystemLibrary.PrintString` "No Cassette to play"))))

(event `/Game/3DGD/BluePrints/Interfaces/BPI_Interactable.UnHover`
  ; Logic for cassette player
  ;; Hover and unhover highlight
  (`PrimitiveComponent.SetRenderCustomDepth` (`self.Cube`) false))

(event `/Game/3DGD/BluePrints/Interfaces/BPI_Interactable.OnHover`
  ; Logic for cassette player
  ;; Hover and unhover highlight
  (`PrimitiveComponent.SetRenderCustomDepth` (`self.Cube`) true))

(fn `UserConstructionScript`)