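; BP_InspectableItem is a world item that highlights on hover and opens an inspection UI when interacted with.
; Construction copies the Cone component's mesh and relative transform onto InspectableMesh.
; Hover events toggle custom depth rendering on Cone.
; Interaction sets the SceneCaptureComponent2D sort priority, creates the Inspect_UI widget, shows the cursor and switches to Game and UI input.
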(event `/Game/3DGD/BluePrints/Interfaces/BPI_Interactable.InteractWithObject`
  (`SceneCaptureComponent.SetCaptureSortPriority` (`self.SceneCaptureComponent2D`) 0)
  (bind _returnvalue (`|CreateWidget` "/Game/3DGD/BluePrints/Inspect_UI.Inspect_UI_C"))
  (bind _output_get (set `self.Inspect UI` _returnvalue))
  (`UserWidget.AddToViewport` _output_get 0)
  (set `PlayerController.bShowMouseCursor` true (`GameplayStatics.GetPlayerController` 0))
  (`WidgetBlueprintLibrary.SetInputMode_GameAndUIEx` null null "DoNotLock" false))

(event `/Game/3DGD/BluePrints/Interfaces/BPI_Interactable.UnHover`
  (`PrimitiveComponent.SetRenderCustomDepth` (`self.Cone`) false))

(event `/Game/3DGD/BluePrints/Interfaces/BPI_Interactable.OnHover`
  (`PrimitiveComponent.SetRenderCustomDepth` (`self.Cone`) true))

(fn `UserConstructionScript`
  (bind _cone (`self.Cone`))
  (bind _inspectable_mesh (`self.inspectable mesh`))
  (`StaticMeshComponent.SetStaticMesh` _inspectable_mesh (`StaticMeshComponent.StaticMesh` _cone))
  (`SceneComponent.K2_SetRelativeTransform` _inspectable_mesh (`SceneComponent.GetRelativeTransform` _cone) false false))