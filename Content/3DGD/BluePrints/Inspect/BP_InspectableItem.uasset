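; BP_InspectableItem is a world object that highlights on hover through custom depth and opens a close-up inspection mode on interaction.
; Its construction script copies the Cone mesh to a hidden duplicate placed far below, which a SceneCaptureComponent2D renders exclusively.
; Interacting shows the duplicate and Inspect_UI, switches the player controller's input context and registers itself there.
; Rotation and FOV-based zoom events manipulate the view, and exiting restores defaults.
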(event `/Game/3DGD/BluePrints/Interfaces/BPI_Interactable.InteractWithObject`
  (bind _returnvalue (`GameplayStatics.GetPlayerController` 0))
  ; BP_Inspecting
  (`SceneCaptureComponent.SetCaptureSortPriority` (`self.SceneCaptureComponent2D`) 0)
  (`SceneComponent.SetHiddenInGame` (`self.inspectable mesh`) false false)
  (bind _returnvalue_2 (`|CreateWidget` "/Game/3DGD/BluePrints/Inspect/InspectTools/Inspect_UI.Inspect_UI_C"))
  (bind _output_get (set `self.Inspect UI` _returnvalue_2))
  (`UserWidget.AddToViewport` _output_get 0)
  (set `PlayerController.bShowMouseCursor` true _returnvalue)
  (`WidgetBlueprintLibrary.SetInputMode_GameAndUIEx` _returnvalue null "DoNotLock" false)
  (bind _asbp_first_person_player_controller (cast `/Game/FirstPerson/Blueprints/BP_FirstPersonPlayerController` (`GameplayStatics.GetPlayerController` 0)))
  (`/Game/FirstPerson/Blueprints/BP_FirstPersonPlayerController.UpdateInputMapContext` _asbp_first_person_player_controller "/Game/Input/IMC_Inspection.IMC_Inspection")
  (set `/Game/FirstPerson/Blueprints/BP_FirstPersonPlayerController.InspectableBP` self _asbp_first_person_player_controller))

(event `Exit Inspect Mode`
  (bind _returnvalue (`GameplayStatics.GetPlayerController` 0))
  (`self.Reset inspectable mesh`)
  (`SceneComponent.SetHiddenInGame` (`self.inspectable mesh`) true false)
  (`Widget.RemoveFromParent` (`self.Inspect UI`))
  (set `PlayerController.bShowMouseCursor` false _returnvalue)
  (`WidgetBlueprintLibrary.SetInputMode_GameOnly` _returnvalue)
  (bind _asbp_first_person_player_controller (cast `/Game/FirstPerson/Blueprints/BP_FirstPersonPlayerController` (`GameplayStatics.GetPlayerController` 0)))
  (`/Game/FirstPerson/Blueprints/BP_FirstPersonPlayerController.UpdateInputMapContext` _asbp_first_person_player_controller "/Game/Input/IMC_Default.IMC_Default"))

(event `UpdateMeshZoom`
  (params (Axis :type "Float (double-precision)"))
  ; Zoom Functionality
  (set `SceneCaptureComponent2D.FOVAngle` (+ (`SceneCaptureComponent2D.FOVAngle` (`self.SceneCaptureComponent2D`)) (* Axis -3.0)) (`self.SceneCaptureComponent2D`))
  (`KismetSystemLibrary.PrintString` (`KismetStringLibrary.Conv_DoubleToString` Axis)))

(event `/Game/3DGD/BluePrints/Interfaces/BPI_Interactable.UnHover`
  ; Highlight and unhighlight inspectable object
  (`PrimitiveComponent.SetRenderCustomDepth` (`self.Cone`) false))

(event `/Game/3DGD/BluePrints/Interfaces/BPI_Interactable.OnHover`
  ; Highlight and unhighlight inspectable object
  (`PrimitiveComponent.SetRenderCustomDepth` (`self.Cone`) true))

(event `Reset inspectable mesh`
  (`SceneComponent.K2_SetRelativeTransform` (`self.inspectable mesh`) (`self.InspectableDefaultPos`) false false)
  (set `SceneCaptureComponent2D.FOVAngle` 90.0 (`self.SceneCaptureComponent2D`))
  (`SceneCaptureComponent.SetCaptureSortPriority` (`self.SceneCaptureComponent2D`) 1))

(event `Update Mesh Rotation`
  (params (`Vector 2D` :type "Vector2D Structure"))
  (bind (_x _y) (`KismetMathLibrary.BreakVector2D` `Vector 2D`))
  (bind _inspectable_mesh (`self.inspectable mesh`))
  ; Update mouse position on drag
  (`SceneComponent.K2_SetRelativeRotation` _inspectable_mesh (`KismetMathLibrary.ComposeRotators` (`SceneComponent.RelativeRotation` _inspectable_mesh) (`KismetMathLibrary.MakeRotator` (* _y -5.0) 0.0 (* _x -5.0))) false false))

(fn `UserConstructionScript`
  (bind _inspectable_mesh (`self.inspectable mesh`))
  (bind _inspectable_mesh_2 (`self.inspectable mesh`))
  (bind _scenecapturecomponent2d (`self.SceneCaptureComponent2D`))
  (bind _cone (`self.Cone`))
  (bind (_relativelocation_x _relativelocation_y) (`KismetMathLibrary.BreakVector` (`SceneComponent.RelativeLocation` _inspectable_mesh)))
  (bind (_relativelocation_x_2 _relativelocation_y_2) (`KismetMathLibrary.BreakVector` (`SceneComponent.RelativeLocation` _scenecapturecomponent2d)))
  (`SceneCaptureComponent.ShowOnlyComponent` (`self.SceneCaptureComponent2D`) (`self.inspectable mesh`))
  (`StaticMeshComponent.SetStaticMesh` _inspectable_mesh_2 (`StaticMeshComponent.StaticMesh` _cone))
  (`SceneComponent.K2_SetRelativeTransform` _inspectable_mesh_2 (`SceneComponent.GetRelativeTransform` _cone) false false)
  (`SceneComponent.K2_SetRelativeLocation` _inspectable_mesh (`KismetMathLibrary.MakeVector` _relativelocation_x _relativelocation_y -1000.0) false false)
  (`SceneComponent.K2_SetRelativeLocation` _scenecapturecomponent2d (`KismetMathLibrary.MakeVector` _relativelocation_x_2 _relativelocation_y_2 -1000.0) false false)
  (set `self.InspectableDefaultPos` (`SceneComponent.GetRelativeTransform` (`self.inspectable mesh`))))