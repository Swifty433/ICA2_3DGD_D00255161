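; BP_PhoneInteraction is an interactable phone whose audio the player can switch on and off.
; The E key and InteractwithObject share one FlipFlop that alternately plays and stops PhoneAudio, printing a debug message each time.
; OnHover and UnHover toggle custom depth rendering on the phone mesh as a highlight hook.
; The collision box overlap events are empty, and the EnableInput and DisableInput nodes are left unconnected.
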(event `self.CollisionBox.OnComponentBeginOverlap`
  (params (OverlappedComponent :type "PrimitiveComponent Object Reference") (OtherActor :type "Actor Object Reference") (OtherComp :type "PrimitiveComponent Object Reference") (OtherBodyIndex :type Integer) (bFromSweep :type Boolean) (SweepResult :type "HitResult Structure (by ref)"))
  ;[0.9323 0.08657 0.2343 0.5] Player Input on and off if in collison box
)

(event `self.CollisionBox.OnComponentEndOverlap`
  (params (OverlappedComponent :type "PrimitiveComponent Object Reference") (OtherActor :type "Actor Object Reference") (OtherComp :type "PrimitiveComponent Object Reference") (OtherBodyIndex :type Integer))
  ;[0.9323 0.08657 0.2343 0.5] Player Input on and off if in collison box
)

(event `Key|E`
  (params (Key :type "Key Structure"))
  ;[0 1 0.6698 0.5] On or off for the audio component
  (:`Pressed`
    (`/Engine/EditorBlueprintResources/StandardMacros.FlipFlop` :!label _label
      (:`A`
        (`AudioComponent.Play` (`self.PhoneAudio`) 0.0)
        (`KismetSystemLibrary.PrintString` "Object Interacted" true true (struct :`G` 0.763156 :`B` 1.0 :`A` 1.0)))
      (:`B`
        (`AudioComponent.Stop` (`self.PhoneAudio`))
        (`KismetSystemLibrary.PrintString` "Object stopped" true true (struct :`G` 0.763156 :`B` 1.0 :`A` 1.0))))))

(event `/Game/3DGD/BluePrints/Interfaces/BPI_Interactable.InteractWithObject`
  (goto _label))

(event `/Game/3DGD/BluePrints/Interfaces/BPI_Interactable.UnHover`
  (`PrimitiveComponent.SetRenderCustomDepth` (`self.PhoneMesh`) false))

(event `/Game/3DGD/BluePrints/Interfaces/BPI_Interactable.OnHover`
  (`PrimitiveComponent.SetRenderCustomDepth` (`self.PhoneMesh`) true))

(fn `UserConstructionScript`)